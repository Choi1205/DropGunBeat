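; BP_EnemyBase is an enemy base that moves to a target point and then fires a limited number of bullets.
; BeginPlay fills HP and skips movement if the target vector is zero.
; Tick applies movement input toward the target and snaps to it when close, setting the arrival flag.
; Once arrived, a cooldown timer spawns BP_BulletActor at FirePoint until the shot counter reaches its limit.
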(event EventBeginPlay
  (Variables|Default|SetcurrentHP (Variables|Default|GetmaxHP)) ; 시작하면 현재 HP를 최대 HP로 초기화
  (if (Utilities|Operators|EqualEqual (Math|Vector|VectorZero) (Variables|Default|GettargetVector) 0.0)
    (Variables|Default|SetisMovingEnd true)))

(event EventTick
  (params (DeltaSeconds :type Float%20%28single-precision%29))
  (bind _firepoint (Variables|Default|GetFirePoint))
  (Utilities|FlowControl|Sequence
    (:then_0
      (if (Variables|Default|GetisMovingEnd)
        (if (> (Variables|Default|GetnumToFire) (Variables|Default|GetfireCounter))
          (bind _output_get (Variables|Default|SetfireTimer (+ DeltaSeconds (Variables|Default|GetfireTimer))))
          (if (> _output_get (Variables|Default|GetfireCooldown))
            (Variables|Default|SetfireTimer 0.0)
            (Game|SpawnActorfromClass "/Game/Choi/BP_BulletActor.BP_BulletActor_C" (Math|Transform|MakeTransform (Transformation|GetWorldLocation _firepoint) (Transformation|GetWorldRotation _firepoint) "1.000000,1.000000,1.000000") "Undefined" "MultiplyWithRoot" 0 0)
            (Variables|Default|SetfireCounter (+ (Variables|Default|GetfireCounter) 1))))
        (else
          (Pawn|Input|AddMovementInput (Math|Vector|Normalize (- (Variables|Default|GettargetVector) (Transformation|GetActorLocation))) 1.0 false))))
    (:then_1
      (if (< (Math|Vector|Distance(Vector) (Transformation|GetActorLocation) (Variables|Default|GettargetVector)) 25.0)
        (Transformation|SetActorLocation (Variables|Default|GettargetVector) false false)
        (Variables|Default|SetisMovingEnd true)))))

(fn ConstructionScript)