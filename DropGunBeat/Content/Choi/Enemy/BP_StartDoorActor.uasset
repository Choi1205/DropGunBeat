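; BP_StartDoorActor is a two-panel sliding door that opens when the player enters its trigger box.
; On Box overlap it casts the other actor to BP_Player, and a DoOnce plays the DoorOpen timeline a single time.
; The timeline track moves Plane and Plane1 apart along relative Y, and nothing in the graph closes or resets the door.
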(event OnComponentBeginOverlap(Box)
  (params (OverlappedComponent :type Primitive%20Component%20Object%20Reference) (OtherActor :type Actor%20Object%20Reference) (OtherComp :type Primitive%20Component%20Object%20Reference) (OtherBodyIndex :type Integer) (bFromSweep :type Boolean) (SweepResult :type Hit%20Result%20Structure%20%28by%20ref%29))
  (bind _plane (Variables|Default|GetPlane))
  (bind _plane1 (Variables|Default|GetPlane1))
  (bind _relativelocation (Variables|/Script/Engine.SceneComponent|GetRelativeLocation _plane))
  (bind _relativelocation_2 (Variables|/Script/Engine.SceneComponent|GetRelativeLocation _plane1))
  (Utilities|Casting|CastToBP_Player OtherActor)
  (Utilities|FlowControl|DoOnce false
    (:Completed
      (bind _newtrack_0 (Timeline|DoorOpen Play)
        (:Update
          (Transformation|SetRelativeLocation _plane (Math|Vector|MakeVector (.x _relativelocation) (+ (* _newtrack_0 -135.0) -1e+02) (.z _relativelocation)) false false)
          (Transformation|SetRelativeLocation _plane1 (Math|Vector|MakeVector (.x _relativelocation_2) (+ (* _newtrack_0 135.0) 1e+02) (.z _relativelocation_2)) false false))))))

(event EventBeginPlay)

(event Collision|EventActorBeginOverlap
  (params (OtherActor :type Actor%20Object%20Reference)))

(event EventTick
  (params (DeltaSeconds :type Float%20%28single-precision%29)))

(fn ConstructionScript)