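; Trigger actor that plays a timed red-fade-to-blackout camera sequence when BP_Player enters its Box.
; On overlap, it starts a ten-second fade toward half-opacity red and shows the cube on the BP_BBKKMusic actor found at BeginPlay.
; Afterwards it hides the cube and snaps the camera to black, then clears the fade a second later.
; Nothing disables the trigger, so it can fire again.
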(event OnComponentBeginOverlap(Box)
  (params (OverlappedComponent :type Primitive%20Component%20Object%20Reference) (OtherActor :type Actor%20Object%20Reference) (OtherComp :type Primitive%20Component%20Object%20Reference) (OtherBodyIndex :type Integer) (bFromSweep :type Boolean) (SweepResult :type Hit%20Result%20Structure%20%28by%20ref%29))
  (Utilities|Casting|CastToBP_Player OtherActor)
  (CameraFades|StartCameraFade (Variables|/Script/Engine.PlayerController|GetPlayerCameraManager (Game|GetPlayerController 0)) 0.0 0.5 1e+01 "(R=1.000000,G=0.000000,B=0.000000,A=1.000000)" false false)
  (Default|SetCubeVisible (Variables|Default|GetMusicActor) true)
  (Utilities|FlowControl|Delay 1e+01)
  (Class|PlayerCameraManager|SetManualCameraFade :self (Variables|/Script/Engine.PlayerController|GetPlayerCameraManager (Game|GetPlayerController 0)) :InFadeAmount 1.0)
  (Default|SetCubeVisible (Variables|Default|GetMusicActor) false)
  (Utilities|FlowControl|Delay 1.0)
  (Class|PlayerCameraManager|SetManualCameraFade :self (Variables|/Script/Engine.PlayerController|GetPlayerCameraManager (Game|GetPlayerController 0))))

(event EventBeginPlay
  (bind _returnvalue (Actor|GetActorOfClass "/Game/Choi/EtcActor/BP_BBKKMusic.BP_BBKKMusic_C"))
  (Variables|Default|SetMusicActor _returnvalue))

(event Collision|EventActorBeginOverlap
  (params (OtherActor :type Actor%20Object%20Reference)))

(event EventTick
  (params (DeltaSeconds :type Float%20%28single-precision%29)))

(fn ConstructionScript)