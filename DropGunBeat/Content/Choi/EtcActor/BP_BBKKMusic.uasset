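; Music visualizer actor that spawns a row of BP_SoundCube actors along world Y and scales them to the music's spectrum.
; On BeginPlay it caches the track duration, gathers every BP_SoundCube in the level and hides their meshes.
; A playback-percent event, re-bound every Tick, converts progress to seconds and samples pre-analyzed Constant-Q NRT data.
; Each channel-0 band sets the Z scale of the cube with the same index.
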(event Custom|PlaybackPercent
  (params (PlayingSoundWave :type Sound%20Wave%20Object%20Reference) (PlaybackPercent :type Float%20%28single-precision%29))
  (CallFunction|ScaleCubes (Variables|Default|GetMusicDuration) PlaybackPercent (Variables|Default|GetCubes)))

(event EventBeginPlay
  (Variables|Default|SetMusicDuration (Variables|/Script/Engine.SoundBase|GetDuration (Variables|/Script/Engine.AudioComponent|GetSound (Variables|Default|GetaudioComp))))
  (bind _cubes (CallFunction|SpawnSoundCubes (Variables|Default|GetNum%20Of%20Cubes) (Variables|Default|GetCube%20Space)))
  (Variables|Default|SetCubes _cubes)
  (CallFunction|SetCubeVisible false))

(event EventTick
  (params (DeltaSeconds :type Float%20%28single-precision%29))
  (EventDispatchers|BindEventtoOnAudioPlaybackPercent (Variables|Default|GetaudioComp) (delegate Custom|PlaybackPercent)))

(fn ConstructionScript)

(fn SpawnSoundCubes
  (params (NumOfCubes :type Integer) (CubeSpace :type Float%20%28double-precision%29))
  (bind _rootcomp (Variables|Default|GetrootComp))
  (bind _returnvalue (Transformation|GetWorldLocation _rootcomp))
  (for _index (range 0 NumOfCubes)
    (Game|SpawnActorfromClass "/Game/Choi/EtcActor/BP_SoundCube.BP_SoundCube_C" (Math|Transform|MakeTransform (Math|Vector|MakeVector (.x _returnvalue) (+ (* _index CubeSpace) (.y _returnvalue)) (.z _returnvalue)) "0, 0, 0" "1.000000,1.000000,1.000000") "Undefined" "MultiplyWithRoot" 0 0))
  (bind _outactors (Actor|GetAllActorsOfClass "/Game/Choi/EtcActor/BP_SoundCube.BP_SoundCube_C"))
  (return _outactors))

(fn SetCubeVisible
  (params (Visible :type Boolean))
  (for _array_element (Variables|Default|GetCubes)
    (Rendering|SetVisibility (Variables|/Game/Choi/EtcActor/BP_SoundCube.BP_SoundCube_C|GetStaticMesh _array_element) Visible false)))

(fn ScaleCubes
  (params (MusicDuration :type Float%20%28double-precision%29) (PercentagePlayed :type Float%20%28double-precision%29) (Cubes :type Array%20of%20BP%20Sound%20Cube%20Object%20References))
  (bind _output_get (LocalVariables|SetAudioPos (* MusicDuration PercentagePlayed)))
  (bind _output_get_2 (LocalVariables|SetFreqStrangth (Class|ConstantQNRT|GetNormalizedChannelConstantQatTime (LocalVariables|GetNRT) _output_get)))
  (for (_array_element _array_index) _output_get_2
    (Transformation|SetWorldScale3D (Variables|/Game/Choi/EtcActor/BP_SoundCube.BP_SoundCube_C|GetStaticMesh (Utilities|Array|Get(acopy) Cubes _array_index)) (Math|Vector|MakeVector (.x (Transformation|GetWorldScale (Variables|/Game/Choi/EtcActor/BP_SoundCube.BP_SoundCube_C|GetStaticMesh (Utilities|Array|Get(acopy) Cubes _array_index)))) (.y (Transformation|GetWorldScale (Variables|/Game/Choi/EtcActor/BP_SoundCube.BP_SoundCube_C|GetStaticMesh (Utilities|Array|Get(acopy) Cubes _array_index)))) (* _array_element (LocalVariables|GetScale))))))