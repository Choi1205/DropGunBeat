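; BP_Platform is an actor that moves along a spline path over a configurable travel time.
; On BeginPlay it finds a BP_Spline actor in the level and plays the MoveObj timeline at a rate derived from TimeToComplete.
; Each update offsets the timeline value by StartPosition, wraps it past one, and places the actor at that fraction of the spline's length in world space.
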(event Custom|MovePlatfrom
  (bind _spline (Variables|Default|GetSpline))
  (bind _spline_2 (Variables|/Game/Choi/EtcActor/BP_Spline.BP_Spline_C|GetSpline _spline))
  (Components|Timeline|SetPlayRate (Variables|Default|GetMoveObj) (/ 1.0 (Variables|Default|GettimeToComplete)))
  (bind _movement (Timeline|MoveObj Play)
    (:Update
      (bind _output_get (Variables|Default|SetAlpha (+ _movement (Variables|Default|GetstartPosition))))
      (if (> _output_get 1.0)
        (Variables|Default|SetAlpha (- (Variables|Default|GetAlpha) 1.0)))
      (Transformation|SetActorTransform (Math|Transform|MakeTransform (Spline|GetLocationatDistanceAlongSpline _spline_2 (Math|Float|Lerp 0.0 (Spline|GetSplineLength _spline_2) (Variables|Default|GetAlpha)) "World") "0, 0, 0" "1.000000,1.000000,1.000000")))))

(event EventBeginPlay
  (bind _returnvalue (Actor|GetActorOfClass "/Game/Choi/EtcActor/BP_Spline.BP_Spline_C"))
  (Variables|Default|SetSpline _returnvalue)
  (CallFunction|MovePlatfrom))

(fn ConstructionScript)