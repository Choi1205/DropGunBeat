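; Start trigger actor for a music level that kicks off play when BP_Player first overlaps its box.
; A Scan timeline drives the actor's Z and ping-pongs endlessly through a FlipFlop.
; The one-shot overlap sets the player's start location, fades the camera in, then after a delay sets Start.
; It then starts BBKK or NightTheater music according to the game instance flag; video-opening nodes are unconnected.
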(event OnComponentBeginOverlap(Box)
  (params (OverlappedComponent :type Primitive%20Component%20Object%20Reference) (OtherActor :type Actor%20Object%20Reference) (OtherComp :type Primitive%20Component%20Object%20Reference) (OtherBodyIndex :type Integer) (bFromSweep :type Boolean) (SweepResult :type Hit%20Result%20Structure%20%28by%20ref%29))
  (bind _asbp_player (Utilities|Casting|CastToBP_Player OtherActor))
  (Utilities|FlowControl|DoOnce false
    (:Completed
      (Class|GunPlayer|SetStartLoc _asbp_player)
      (CameraFades|StartCameraFade :self (Variables|/Script/Engine.PlayerController|GetPlayerCameraManager (Game|GetPlayerController 0)) :FromAlpha 1.0 :Duration 2.0)
      (Utilities|FlowControl|Delay 2.0)
      (Variables|/Script/DropGunBeat.GunPlayer|SetbStart _asbp_player true)
      (bind _asbp_music_game_instance (Utilities|Casting|CastToBP_MusicGameInstance (Game|GetGameInstance)))
      (if (Variables|/Script/DropGunBeat.musicGameInstance|GetbIsPlaingBBKK _asbp_music_game_instance)
        (bind _outactors (Actor|GetAllActorsOfClass "/Game/Choi/EtcActor/BP_BBKKMusic.BP_BBKKMusic_C"))
        (Class|MusicActor|MusicStart (Utilities|Array|Get(acopy) _outactors))
        (else
          (bind _outactors_2 (Actor|GetAllActorsOfClass "/Game/Choi/EtcActor/BP_NightTheaterMusic.BP_NightTheaterMusic_C"))
          (Class|MusicActor|MusicStart (Utilities|Array|Get(acopy) _outactors_2)))))))

(event EventBeginPlay
  (bind _returnvalue (Transformation|GetActorLocation))
  (bind _cheak (Timeline|Scan PlayFromStart)
    (:Update
      (Transformation|SetActorLocation (Math|Vector|MakeVector (.x _returnvalue) (.y _returnvalue) _cheak) false false))
    (:Finished
      (Utilities|FlowControl|FlipFlop
        (:A
          (Timeline|Scan ReverseFromEnd))
        (:B
          (Timeline|Scan PlayFromStart))))))

(event Collision|EventActorBeginOverlap
  (params (OtherActor :type Actor%20Object%20Reference)))

(event EventTick
  (params (DeltaSeconds :type Float%20%28single-precision%29)))

(fn ConstructionScript)